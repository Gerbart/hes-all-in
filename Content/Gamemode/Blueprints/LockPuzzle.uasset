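; Clickable lock puzzle actor for point-and-click play that opens a code-entry widget and clears linked objects when solved.
; Clicking its collision plays a sound, creates the lock UI with itself as LockActor and switches to UI-only input.
; Exiting or entering the correct code removes the widget and restores Game-and-UI input.
; Success also destroys up to four HideObjects through chained validity checks, with the locker-open sound requiring all four.
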(event `self.ReceiveActorOnClicked`
  (params (ButtonPressed :type "Key Structure"))
  (`AudioComponent.Play` (`self.ClickNoise`) 0.0)
  (cast `/Game/Gamemode/Blueprints/BP_PnC_MouseController` (`GameplayStatics.GetPlayerController` 0)))

(event `/Game/Gamemode/Blueprints/BPI_LockUICommunication.OnUnlockSuccess`)

(event `self.ReceiveActorBeginCursorOver`
  (set `PlayerController.CurrentMouseCursor` "Hand" (`GameplayStatics.GetPlayerController` 0)))

(event `self.ReceiveActorEndCursorOver`
  (set `PlayerController.CurrentMouseCursor` "Default" (`GameplayStatics.GetPlayerController` 0)))

(event `self.ClickCollision.OnClicked`
  (params (TouchedComponent :type "PrimitiveComponent Object Reference") (ButtonPressed :type "Key Structure"))
  (`AudioComponent.Play` (`self.ClickNoise`) 0.0)
  (bind _returnvalue (`|CreateWidget` (`self.LockUIClass`) null self))
  (bind _output_get (set `self.LockUI` _returnvalue))
  (`UserWidget.AddToViewport` _output_get 0)
  (`WidgetBlueprintLibrary.SetInputMode_UIOnlyEx` (`GameplayStatics.GetPlayerController` 0) (`self.LockUI`))
  (set `PlayerController.bShowMouseCursor` true (`GameplayStatics.GetPlayerController` 0)))

(event `/Game/Gamemode/Blueprints/BPI_LockUICommunication.OnExitLock`
  (`Widget.RemoveFromParent` (`self.LockUI`))
  (set `self.LockUI` null)
  (`WidgetBlueprintLibrary.SetInputMode_GameAndUIEx` (`GameplayStatics.GetPlayerController` 0) null "DoNotLock" false)
  (cast `/Game/Gamemode/Blueprints/BP_PnC_MouseController` (`GameplayStatics.GetPlayerController` 0))
  (set `PlayerController.bShowMouseCursor` true (`GameplayStatics.GetPlayerController` 0)))

(event `CustomEvent`
  (set `PlayerController.CurrentMouseCursor` "Hand" (`GameplayStatics.GetPlayerController` 0)))

(event `CustomEvent_1`
  (set `PlayerController.CurrentMouseCursor` "Default" (`GameplayStatics.GetPlayerController` 0)))

(event `/Game/Gamemode/Blueprints/BPI_LockUICommunication.CorrectCodeEntered`
  (bind _hideobject3 (`self.HideObject3`))
  (bind _hideobject4 (`self.HideObject4`))
  (bind _hideobject1 (`self.HideObject1`))
  (bind _hideobject2 (`self.HideObject2`))
  (`GameplayStatics.PlaySound2D` "/Game/Audio/Sound_Effects/HAI_SFX_PuzzleSolvedTune.HAI_SFX_PuzzleSolvedTune" 1.0 1.0 0.0 null null)
  (`Widget.RemoveFromParent` (`self.LockUI`))
  (set `self.LockUI` null)
  (`WidgetBlueprintLibrary.SetInputMode_GameAndUIEx` (`GameplayStatics.GetPlayerController` 0) null "DoNotLock" false)
  (set `PlayerController.bShowMouseCursor` true (`GameplayStatics.GetPlayerController` 0))
  (`WidgetBlueprintLibrary.SetFocusToGameViewport`)
  (if (`KismetSystemLibrary.IsValid` _hideobject1)
    (`self.K2_DestroyActor` _hideobject1)
    (if (`KismetSystemLibrary.IsValid` _hideobject2)
      (`self.K2_DestroyActor` _hideobject2)
      (if (`KismetSystemLibrary.IsValid` _hideobject3)
        (`self.K2_DestroyActor` _hideobject3)
        (if (`KismetSystemLibrary.IsValid` _hideobject4)
          (`self.K2_DestroyActor` _hideobject4)
          (`GameplayStatics.PlaySound2D` "/Game/Audio/Sound_Effects/HAI_SFX_OpenLocker.HAI_SFX_OpenLocker" 1.0 1.0 0.0 null null))))))

(fn `UserConstructionScript`)