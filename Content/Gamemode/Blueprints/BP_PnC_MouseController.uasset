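; Player controller for a point-and-click game that handles static camera views, dialogue playback and inventory pickups.
; It starts on a static camera in the level and can switch the view target to any camera passed in.
; Dialogue shows a widget, steps through an array of lines on continue clicks with audio, then removes it and restores the cursor.
; Given items become slot widgets with an image and name, added to the inventory HUD panel.
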(event `self.ReceiveBeginPlay`
  (bind _returnvalue (`GameplayStatics.GetActorOfClass` "/Game/Gamemode/Blueprints/BP_StaticCamera.BP_StaticCamera_C"))
  (`self.SetViewTargetWithBlend` _returnvalue))

(event `Advance Dialogue`
  (bind _dialogue_widget (`self.Dialogue Widget`))
  (bind _lines (`self.Lines`))
  (add `/Game/Gamemode/Blueprints/WBP_Dialogue.ClickedToContinue` (`self.Dialogue Widget`) (delegate `Advance Dialogue`))
  (bind _result (`/Engine/EditorBlueprintResources/StandardMacros.IncrementInt` (`self.Current Line`))
    (:`  `
      (if (`KismetArrayLibrary.Array_IsValidIndex` _lines _result)
        (bind _output_get (set `self.Current Line` _result))
        (set `/Game/Gamemode/Blueprints/WBP_Dialogue.String` (`|GetArrayItem` _lines _output_get) _dialogue_widget)
        (`AudioComponent.Play` (`self.Dialogue Audio`) 0.0)
        (else
          (set `self.Current Line` -1)
          (`Widget.RemoveFromParent` _dialogue_widget)
          (`KismetSystemLibrary.CollectGarbage`)
          (set `self.bShowMouseCursor` true)
          (set `self.Dialogue Finished` true))))))

(fn `Give Item`
  (params (`Item Picture` :type "Texture2D Object Reference") (`Item Name` :type Name))
  (bind _returnvalue (`|CreateWidget` "/Game/Gamemode/Blueprints/WBP_ItemSlot.WBP_ItemSlot_C"))
  (bind _output_get (set `self.Item Widget` _returnvalue))
  (`Image.SetBrush` (`/Game/Gamemode/Blueprints/WBP_ItemSlot.ItemImage` _output_get) (make `SlateBrush` (struct :`SpecifiedColor` (struct :`R` 1.0 :`G` 1.0 :`B` 1.0 :`A` 1.0) :`ColorUseRule` "UseColor_Specified") "Image" "NoTile" "NoMirror" (`KismetMathLibrary.MakeVector2D` 140.0 140.0) (make `Margin` 5.0 5.0 5.0 5.0) `Item Picture`))
  (set `/Game/Gamemode/Blueprints/WBP_ItemSlot.Item Name` `Item Name` (`self.Item Widget`))
  (bind _foundwidgets (`WidgetBlueprintLibrary.GetAllWidgetsOfClass` "/Game/Gamemode/Blueprints/WBP_InventoryHUD.WBP_InventoryHUD_C"))
  (`PanelWidget.AddChild` (`/Game/Gamemode/Blueprints/WBP_InventoryHUD.InventoryPanel` (`|GetArrayItem` _foundwidgets)) (`self.Item Widget`)))

(fn `Play Dialogue`
  (params (Lines :type "Array of String"))
  (set `self.Dialogue Finished` false)
  (bind _output_get (set `self.Lines` Lines))
  (bind _returnvalue (`|CreateWidget` "/Game/Gamemode/Blueprints/WBP_Dialogue.WBP_Dialogue_C"))
  (set `/Game/Gamemode/Blueprints/WBP_Dialogue.String` (`|GetArrayItem` _output_get (`self.Current Line`)) _returnvalue)
  (bind _output_get_2 (set `self.Dialogue Widget` _returnvalue))
  (`UserWidget.AddToViewport` _output_get_2 0)
  (`AudioComponent.Play` (`self.Dialogue Audio`) 0.0)
  (set `self.bShowMouseCursor` false)
  (`WidgetBlueprintLibrary.SetInputMode_GameAndUIEx` (`GameplayStatics.GetPlayerController` 0) _returnvalue "LockAlways")
  (`self.Advance Dialogue`)
  (return))

(fn `Swap Camera`
  (params (`Input Camera` :type "CameraActor Object Reference"))
  (`self.SetViewTargetWithBlend` `Input Camera`))

(fn `UserConstructionScript`)