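; Clickable janitor door in the Laundromat level of a point-and-click game, which accepts an inventory item and leads to the next scene.
; Hovering shows a hand cursor; clicking plays a sound and dialogue through BP_PnC_MouseController.
; UseItem plays a sound, then for a matching item removes its slot widget and starts item dialogue.
; Tick then polls for that dialogue to finish before opening CharliesScene.
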(event `self.ReceiveActorOnClicked`
  (params (ButtonPressed :type "Key Structure"))
  (`AudioComponent.Play` (`self.Audio`) 0.0)
  (bind _asbp_pn_c_mouse_controller (cast `/Game/Gamemode/Blueprints/BP_PnC_MouseController` (`GameplayStatics.GetPlayerController` 0)))
  (`/Game/Gamemode/Blueprints/BP_PnC_MouseController.Play Dialogue` _asbp_pn_c_mouse_controller (`self.Lines`)))

(event `self.ReceiveActorBeginCursorOver`
  (set `PlayerController.CurrentMouseCursor` "Hand" (`GameplayStatics.GetPlayerController` 0)))

(event `self.ReceiveActorEndCursorOver`
  (set `PlayerController.CurrentMouseCursor` "Default" (`GameplayStatics.GetPlayerController` 0)))

(event `self.UseItem`
  (params (`Item Widget` :type "Widget Object Reference"))
  (`AudioComponent.Play` (`self.Use Item Sound`) 0.0)
  (bind _aswbp_item_slot (cast `/Game/Gamemode/Blueprints/WBP_ItemSlot` `Item Widget`))
  (if (== (`/Game/Gamemode/Blueprints/WBP_ItemSlot.Item Name` _aswbp_item_slot) (`self.Item`))
    (`KismetSystemLibrary.PrintString` "tried key on lock")
    (`Widget.RemoveFromParent` `Item Widget`)
    (`KismetSystemLibrary.CollectGarbage`)
    (bind _asbp_pn_c_mouse_controller (cast `/Game/Gamemode/Blueprints/BP_PnC_MouseController` (`GameplayStatics.GetPlayerController` 0)))
    (`/Game/Gamemode/Blueprints/BP_PnC_MouseController.Play Dialogue` _asbp_pn_c_mouse_controller (`self.Item Lines`))
    (set `self.dialog over` true)))

(event `self.ReceiveTick`
  (params (DeltaSeconds :type "Float (single-precision)"))
  (if (`self.dialog over`)
    (bind _asbp_pn_c_mouse_controller (cast `/Game/Gamemode/Blueprints/BP_PnC_MouseController` (`GameplayStatics.GetPlayerController` 0)))
    (if (`/Game/Gamemode/Blueprints/BP_PnC_MouseController.Dialogue Finished` _asbp_pn_c_mouse_controller)
      (`GameplayStatics.OpenLevel` "CharliesScene"))))

(fn `UserConstructionScript`)