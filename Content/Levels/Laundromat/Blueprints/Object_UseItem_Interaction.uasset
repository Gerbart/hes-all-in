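; Clickable point-and-click object for the Laundromat level that plays dialogue and accepts one matching inventory item.
; Hovering switches the cursor to a hand; clicking plays audio and sends its lines to BP_PnC_MouseController.
; UseItem always plays a sound, then compares the slot widget's item name to the required item.
; A match removes the widget, plays item dialogue and, if a new mesh is set, swaps it onto a replacement actor.
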(event `self.ReceiveActorOnClicked`
  (params (ButtonPressed :type "Key Structure"))
  (`AudioComponent.Play` (`self.Audio`) 0.0)
  (bind _asbp_pn_c_mouse_controller (cast `/Game/Gamemode/Blueprints/BP_PnC_MouseController` (`GameplayStatics.GetPlayerController` 0)))
  (`/Game/Gamemode/Blueprints/BP_PnC_MouseController.Play Dialogue` _asbp_pn_c_mouse_controller (`self.Lines`)))

(event `self.ReceiveActorBeginCursorOver`
  (set `PlayerController.CurrentMouseCursor` "Hand" (`GameplayStatics.GetPlayerController` 0)))

(event `self.ReceiveActorEndCursorOver`
  (set `PlayerController.CurrentMouseCursor` "Default" (`GameplayStatics.GetPlayerController` 0)))

(event `/Game/Gamemode/Blueprints/BPI_Interactable.UseItem`
  (params (`Item Widget` :type "Widget Object Reference"))
  (bind _new_mesh (`self.New Mesh`))
  (`AudioComponent.Play` (`self.Use Item Sound`) 0.0)
  (bind _aswbp_item_slot (cast `/Game/Gamemode/Blueprints/WBP_ItemSlot` `Item Widget`))
  (if (== (`/Game/Gamemode/Blueprints/WBP_ItemSlot.Item Name` _aswbp_item_slot) (`self.Item`))
    (`KismetSystemLibrary.PrintString` "tried key on lock")
    (`Widget.RemoveFromParent` `Item Widget`)
    (`KismetSystemLibrary.CollectGarbage`)
    (bind _asbp_pn_c_mouse_controller (cast `/Game/Gamemode/Blueprints/BP_PnC_MouseController` (`GameplayStatics.GetPlayerController` 0)))
    (`/Game/Gamemode/Blueprints/BP_PnC_MouseController.Play Dialogue` _asbp_pn_c_mouse_controller (`self.Item Lines`))
    (if (`KismetSystemLibrary.IsValid` _new_mesh)
      (`StaticMeshComponent.SetStaticMesh` (`StaticMeshActor.StaticMeshComponent` (`self.Replacement Mesh Actor`)) _new_mesh))))

(fn `UserConstructionScript`)