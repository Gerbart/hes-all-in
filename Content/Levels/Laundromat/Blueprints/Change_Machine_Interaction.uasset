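; Point-and-click interactable for the laundromat change machine that responds to clicks and inventory item use.
; Clicking plays audio and dialogue through BP_PnC_MouseController, and hovering switches the cursor to a hand.
; UseItem always plays a sound, then, if the slot's item name matches, removes that widget, plays item dialogue and gives the player a new item.
; A match also moves a target actor 1000 units up to activate it.
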(event `self.ReceiveActorOnClicked`
  (params (ButtonPressed :type "Key Structure"))
  (`AudioComponent.Play` (`self.Audio`) 0.0)
  (bind _asbp_pn_c_mouse_controller (cast `/Game/Gamemode/Blueprints/BP_PnC_MouseController` (`GameplayStatics.GetPlayerController` 0)))
  (`/Game/Gamemode/Blueprints/BP_PnC_MouseController.Play Dialogue` _asbp_pn_c_mouse_controller (`self.Lines`)))

(event `self.ReceiveActorBeginCursorOver`
  (set `PlayerController.CurrentMouseCursor` "Hand" (`GameplayStatics.GetPlayerController` 0)))

(event `self.ReceiveActorEndCursorOver`
  (set `PlayerController.CurrentMouseCursor` "Default" (`GameplayStatics.GetPlayerController` 0)))

(event `self.UseItem`
  (params (`Item Widget` :type "Widget Object Reference"))
  (bind _target_to_activate (`self.Target to Activate`))
  (`AudioComponent.Play` (`self.Use Item Sound`) 0.0)
  (bind _aswbp_item_slot (cast `/Game/Gamemode/Blueprints/WBP_ItemSlot` `Item Widget`))
  (if (== (`/Game/Gamemode/Blueprints/WBP_ItemSlot.Item Name` _aswbp_item_slot) (`self.Item`))
    (`KismetSystemLibrary.PrintString` "tried key on lock")
    (`Widget.RemoveFromParent` `Item Widget`)
    (`KismetSystemLibrary.CollectGarbage`)
    (bind _asbp_pn_c_mouse_controller (cast `/Game/Gamemode/Blueprints/BP_PnC_MouseController` (`GameplayStatics.GetPlayerController` 0)))
    (`/Game/Gamemode/Blueprints/BP_PnC_MouseController.Play Dialogue` _asbp_pn_c_mouse_controller (`self.Item Lines`))
    (bind _asbp_pn_c_mouse_controller_2 (cast `/Game/Gamemode/Blueprints/BP_PnC_MouseController` (`GameplayStatics.GetPlayerController` 0)))
    (`/Game/Gamemode/Blueprints/BP_PnC_MouseController.Give Item` _asbp_pn_c_mouse_controller_2 (`self.Item Picture`) (`self.Item Name`))
    (`self.K2_SetActorTransform` _target_to_activate (`KismetMathLibrary.MakeTransform` (+ (.location (`self.GetTransform` _target_to_activate)) (0.0 0.0 1000.0)) (.rotation (`self.GetTransform` _target_to_activate)) (.scale (`self.GetTransform` _target_to_activate))) false false)))

(fn `UserConstructionScript`)