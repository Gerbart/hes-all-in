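; Clickable keys pickup for the Laundromat level of a point-and-click game.
; On click, it casts the player controller to BP_PnC_MouseController, plays its dialogue lines, gives the player a "Keys" item with a picture, then destroys itself.
; Hover events switch the mouse cursor to a hand and restore the default on exit.
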(event `self.ReceiveActorOnClicked`
  (params (ButtonPressed :type "Key Structure"))
  (bind _asbp_pn_c_mouse_controller (cast `/Game/Gamemode/Blueprints/BP_PnC_MouseController` (`GameplayStatics.GetPlayerController` 0)))
  (`/Game/Gamemode/Blueprints/BP_PnC_MouseController.Play Dialogue` _asbp_pn_c_mouse_controller (`self.Lines`))
  (`/Game/Gamemode/Blueprints/BP_PnC_MouseController.Give Item` _asbp_pn_c_mouse_controller "/Game/Characters/Mannequins/Textures/Manny/T_Manny_01_MRA.T_Manny_01_MRA" "Keys")
  (`self.K2_DestroyActor`))

(event `self.ReceiveActorBeginCursorOver`
  (set `PlayerController.CurrentMouseCursor` "Hand" (`GameplayStatics.GetPlayerController` 0)))

(event `self.ReceiveActorEndCursorOver`
  (set `PlayerController.CurrentMouseCursor` "Default" (`GameplayStatics.GetPlayerController` 0)))

(fn `UserConstructionScript`)