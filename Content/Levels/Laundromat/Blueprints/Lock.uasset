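; Clickable lock actor in the Laundromat level that shows dialogue and accepts a key from an item slot.
; Clicking creates a WBP_Dialogue widget that steps through the Lines array on each continue click, then resets and closes.
; Hovering switches the cursor to a hand.
; UseItem removes a "Keys" slot widget and forces garbage collection, but only prints a message without changing any lock state.
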(event `self.ReceiveActorOnClicked`
  (params (ButtonPressed :type "Key Structure"))
  (`KismetSystemLibrary.PrintString` "Hello")
  (bind _returnvalue (`|CreateWidget` "/Game/Gamemode/Blueprints/WBP_Dialogue.WBP_Dialogue_C"))
  (set `/Game/Gamemode/Blueprints/WBP_Dialogue.String` (`|GetArrayItem` (`self.Lines`) (`self.Current Line`)) _returnvalue)
  (bind _output_get (set `self.Dialogue Widget` _returnvalue))
  (`UserWidget.AddToViewport` _output_get 0)
  (add `/Game/Gamemode/Blueprints/WBP_Dialogue.ClickedToContinue` _output_get (delegate `Advance Dialogue`)))

(event `Advance Dialogue`
  (bind _dialogue_widget (`self.Dialogue Widget`))
  (bind _lines (`self.Lines`))
  (bind _result (`/Engine/EditorBlueprintResources/StandardMacros.IncrementInt` (`self.Current Line`))
    (:`  `
      (if (`KismetArrayLibrary.Array_IsValidIndex` _lines _result)
        (bind _output_get (set `self.Current Line` _result))
        (set `/Game/Gamemode/Blueprints/WBP_Dialogue.String` (`|GetArrayItem` _lines _output_get) _dialogue_widget)
        (else
          (set `self.Current Line` 0)
          (`Widget.RemoveFromParent` _dialogue_widget))))))

(event `self.ReceiveActorBeginCursorOver`
  (set `PlayerController.CurrentMouseCursor` "Hand" (`GameplayStatics.GetPlayerController` 0)))

(event `self.ReceiveActorEndCursorOver`
  (set `PlayerController.CurrentMouseCursor` "Default" (`GameplayStatics.GetPlayerController` 0)))

(fn `UseItem`
  (params (`Item Widget` :type "Widget Object Reference"))
  (bind _aswbp_item_slot (cast `/Game/Gamemode/Blueprints/WBP_ItemSlot` `Item Widget`))
  (if (== (`/Game/Gamemode/Blueprints/WBP_ItemSlot.Item Name` _aswbp_item_slot) "Keys")
    (`KismetSystemLibrary.PrintString` "tried key on lock")
    (`Widget.RemoveFromParent` `Item Widget`)
    (`KismetSystemLibrary.CollectGarbage`)
    (return)))

(fn `UserConstructionScript`)