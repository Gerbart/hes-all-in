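; Point-and-click washer interactable in the Laundromat level that plays dialogue on click, swaps the hover cursor and accepts a matching inventory item.
; A correct item is removed and triggers dialogue through BP_PnC_MouseController.
; Tick polls DialogueFinished to stage one-shot steps: swap a mesh and show the marked card with final dialogue, then play a sequence.
; When the sequence stops, the BarToCasino level opens.
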(event `self.ReceiveActorOnClicked`
  (params (ButtonPressed :type "Key Structure"))
  (`AudioComponent.Play` (`self.Audio`) 0.0)
  (bind _asbp_pn_c_mouse_controller (cast `/Game/Gamemode/Blueprints/BP_PnC_MouseController` (`GameplayStatics.GetPlayerController` 0)))
  (`/Game/Gamemode/Blueprints/BP_PnC_MouseController.Play Dialogue` _asbp_pn_c_mouse_controller (`self.Lines`)))

(event `self.ReceiveActorBeginCursorOver`
  (set `PlayerController.CurrentMouseCursor` "Hand" (`GameplayStatics.GetPlayerController` 0)))

(event `self.ReceiveActorEndCursorOver`
  (set `PlayerController.CurrentMouseCursor` "Default" (`GameplayStatics.GetPlayerController` 0)))

(event `self.UseItem`
  (params (`Item Widget` :type "Widget Object Reference"))
  (`AudioComponent.Play` (`self.Use Item Sound`) 0.0)
  (bind _aswbp_item_slot (cast `/Game/Gamemode/Blueprints/WBP_ItemSlot` `Item Widget`))
  (if (== (`/Game/Gamemode/Blueprints/WBP_ItemSlot.Item Name` _aswbp_item_slot) (`self.Item Name`))
    (`KismetSystemLibrary.PrintString` "tried key on lock")
    (`Widget.RemoveFromParent` `Item Widget`)
    (`KismetSystemLibrary.CollectGarbage`)
    (bind _asbp_pn_c_mouse_controller (cast `/Game/Gamemode/Blueprints/BP_PnC_MouseController` (`GameplayStatics.GetPlayerController` 0)))
    (`/Game/Gamemode/Blueprints/BP_PnC_MouseController.Play Dialogue` _asbp_pn_c_mouse_controller (`self.Item Lines`))
    (set `self.Used Item Dialogue Finished` true)))

(event `self.ReceiveTick`
  (params (DeltaSeconds :type "Float (single-precision)"))
  (bind _sequenceplayer (`LevelSequenceActor.SequencePlayer` (`self.Sequence`)))
  (bind _asbp_pn_c_mouse_controller (cast `/Game/Gamemode/Blueprints/BP_PnC_MouseController` (`GameplayStatics.GetPlayerController` 0)))
  (if (`/Game/Gamemode/Blueprints/BP_PnC_MouseController.Dialogue Finished` _asbp_pn_c_mouse_controller)
    (if (`self.Viewed Card`)
      (`/Engine/EditorBlueprintResources/StandardMacros.DoOnce` false
        (:`Completed`
          (`Widget.RemoveFromParent` (stale _returnvalue_2))
          (bind _returnvalue (`|CreateWidget` "/Game/Gamemode/Blueprints/Fade_In.Fade_In_C"))
          (`WidgetBlueprintLibrary.SetInputMode_UIOnlyEx` _asbp_pn_c_mouse_controller _returnvalue "LockAlways")
          (set `PlayerController.bShowMouseCursor` false _asbp_pn_c_mouse_controller)
          (`MovieSceneSequencePlayer.Play` _sequenceplayer)
          (add `MovieSceneSequencePlayer.OnStop` _sequenceplayer (delegate `On Stop`))))
      (elif (`self.Used Item Dialogue Finished`)
        (`/Engine/EditorBlueprintResources/StandardMacros.DoOnce` false
          (:`Completed`
            (`AudioComponent.Play` (`self.Use Item Sound 2`) 0.0)
            (`StaticMeshComponent.SetStaticMesh` (`StaticMeshActor.StaticMeshComponent` (`self.Replacement Mesh Actor`)) (`self.New Mesh`))
            (bind _returnvalue_2 (`|CreateWidget` "/Game/Levels/Laundromat/Blueprints/Marked_Card_Screen.Marked_Card_Screen_C"))
            (`UserWidget.AddToViewport` _returnvalue_2 0)
            (`/Game/Gamemode/Blueprints/BP_PnC_MouseController.Play Dialogue` _asbp_pn_c_mouse_controller (`self.Final Lines`))
            (`self.K2_DestroyActor` (`self.delete mesh`))
            (set `self.Viewed Card` true)))))))

(event `On Stop`
  (`GameplayStatics.OpenLevel` "BarToCasino"))

(fn `UserConstructionScript`)