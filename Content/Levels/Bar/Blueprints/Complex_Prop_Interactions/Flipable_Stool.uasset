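; Flipable_Stool is a clickable bar stool prop for the point-and-click controller, swapped for another actor when used.
; Clicking plays dialogue lines through BP_PnC_MouseController, spawns the configured object at a set transform, applies the TableStool1 mesh to it if it is a Stool, then destroys itself.
; Cursor hover switches the player's mouse cursor to a hand and back to default on exit.
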(event `self.ReceiveActorOnClicked`
  (params (ButtonPressed :type "Key Structure"))
  (bind _asbp_pn_c_mouse_controller (cast `/Game/Gamemode/Blueprints/BP_PnC_MouseController` (`GameplayStatics.GetPlayerController` 0)))
  (`/Game/Gamemode/Blueprints/BP_PnC_MouseController.Play Dialogue` _asbp_pn_c_mouse_controller (`self.Lines`))
  (bind _returnvalue (`|SpawnActorFromClass` (`self.Spawn Object`) (`self.Spawn Transform`) "Undefined" "MultiplyWithRoot" null null))
  (bind _asstool (cast `/Game/Levels/Bar/Blueprints/Simple_Prop_Interactions/Stool` _returnvalue))
  (`StaticMeshComponent.SetStaticMesh` (`/Game/Levels/Bar/Blueprints/Simple_Prop_Interactions/Stool.StaticMesh` _asstool) "/Game/Environments/Bar/tableStool1.tableStool1")
  (`self.K2_DestroyActor`))

(event `self.ReceiveActorBeginCursorOver`
  (set `PlayerController.CurrentMouseCursor` "Hand" (`GameplayStatics.GetPlayerController` 0)))

(event `self.ReceiveActorEndCursorOver`
  (set `PlayerController.CurrentMouseCursor` "Default" (`GameplayStatics.GetPlayerController` 0)))

(fn `UserConstructionScript`)