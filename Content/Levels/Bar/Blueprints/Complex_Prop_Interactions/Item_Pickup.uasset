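; Clickable item pickup for a point-and-click game, stored with the Bar level's interactive props.
; Hovering switches the cursor to a hand, restoring the default on exit.
; A click plays audio, then has BP_PnC_MouseController play the item's dialogue lines and receive its name and picture.
; It then destroys the referenced Object actor and itself; both steps are skipped if the controller cast fails.
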(event `self.ReceiveActorOnClicked`
  (params (ButtonPressed :type "Key Structure"))
  (`AudioComponent.Play` (`self.Audio`) 0.0)
  (bind _asbp_pn_c_mouse_controller (cast `/Game/Gamemode/Blueprints/BP_PnC_MouseController` (`GameplayStatics.GetPlayerController` 0)))
  (`/Game/Gamemode/Blueprints/BP_PnC_MouseController.Play Dialogue` _asbp_pn_c_mouse_controller (`self.Lines`))
  (`/Game/Gamemode/Blueprints/BP_PnC_MouseController.Give Item` _asbp_pn_c_mouse_controller (`self.Item Picture`) (`self.Item Name`))
  (`self.K2_DestroyActor` (`self.Object`))
  (`self.K2_DestroyActor`))

(event `self.ReceiveActorBeginCursorOver`
  (set `PlayerController.CurrentMouseCursor` "Hand" (`GameplayStatics.GetPlayerController` 0)))

(event `self.ReceiveActorEndCursorOver`
  (set `PlayerController.CurrentMouseCursor` "Default" (`GameplayStatics.GetPlayerController` 0)))

(fn `UserConstructionScript`)