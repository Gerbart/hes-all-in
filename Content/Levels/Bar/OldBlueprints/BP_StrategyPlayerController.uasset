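; Player controller for a strategy game with mouse and touch Enhanced Input, handling unit selection, group move orders and drag-scrolling.
; Taps sphere-trace for Pawns to toggle in ControlledUnits; holds send drag boxes to the HUD, and double-tap selects on-screen Pawns.
; Move orders send one unit to the goal, others to random navigable points nearby; the first close arrival interacts.
; Camera move, zoom and reset inputs are unwired.
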(event `self.ReceiveBeginPlay`
  (bind _returnvalue (subsystem `EnhancedInputLocalPlayerSubsystem`))
  (`|ExecutionSequence`
    (:`then_0`
      ; Get Starting Orthographic Zoom
      (bind _asbp_strategy_pawn (cast `/Game/Levels/Bar/OldBlueprints/BP_StrategyPawn` (`self.K2_GetPawn`)))
      (bind _orthowidth (`CameraComponent.OrthoWidth` (`/Game/Levels/Bar/OldBlueprints/BP_StrategyPawn.Camera` _asbp_strategy_pawn)))
      (set `self.Camera Zoom` _orthowidth)
      (set `self.ControlledPawn` _asbp_strategy_pawn)
      (set `self.DefaultZoom` _orthowidth))
    (:`then_1`
      ;[0.05098 0.05098 0.05098] Setup Input Mapping
      (`/Engine/EditorBlueprintResources/StandardMacros.IsValid` _returnvalue :!label _label
        (:`Is Valid`
          (switch `/Game/Levels/Bar/Input/Enum_InputModes` (`self.InputModes`)
            (:`NewEnumerator0`
              (`EnhancedInputSubsystemInterface.AddMappingContext` _returnvalue "/Game/Levels/Bar/Input/IMC_Strategy_Mouse.IMC_Strategy_Mouse" 0 (struct)))
            (:`NewEnumerator1`
              (`EnhancedInputSubsystemInterface.AddMappingContext` _returnvalue "/Game/Levels/Bar/Input/IMC_Strategy_Touch.IMC_Strategy_Touch" 0 (struct)))))))))

(event `Set Controls`
  ;[0.05098 0.05098 0.05098] Setup Input Mapping
  (goto _label))

(event `EnhancedInput|/Game/Levels/Bar/Input/Actions/IA_Strategy_SelectHold`
  (params (ActionValue :type Boolean) (ElapsedSeconds :type "Float (double-precision)") (TriggeredSeconds :type "Float (double-precision)") (InputAction :type "InputAction Object Reference" :default "/Game/Levels/Bar/Input/Actions/IA_Strategy_SelectHold.IA_Strategy_SelectHold"))
  (bind (_startingselectionposition_x _startingselectionposition_y) (`KismetMathLibrary.BreakVector2D` (`self.StartingSelectionPosition`)))
  ;[0.15 0.15 0.15 0.502] Selection Logic for Mouse - Select / Drag Select on Hold
  (:`Triggered`
    (bind _mouse_pos (`self.GetMouseLocation`))
    (message `/Game/Levels/Bar/OldBlueprints/BPI_Strategy.DragSelectUpdate` (`self.GetHUD`) (`self.StartingSelectionPosition`) (`KismetMathLibrary.MakeVector2D` (- (`KismetMathLibrary.BreakVector2D` _mouse_pos) _startingselectionposition_x) (- (`.Y` (`KismetMathLibrary.BreakVector2D` _mouse_pos)) _startingselectionposition_y)) (`KismetMathLibrary.MakeVector2D` (`KismetMathLibrary.BreakVector2D` _mouse_pos) (`.Y` (`KismetMathLibrary.BreakVector2D` _mouse_pos))) true))
  (:`Started`
    (bind _mouse_pos_2 (`self.GetMouseLocation`))
    (set `self.StartingSelectionPosition` _mouse_pos_2))
  (:`Canceled`
    (message `/Game/Levels/Bar/OldBlueprints/BPI_Strategy.DragSelectUpdate` (`self.GetHUD`) (0.0 0.0) (0.0 0.0) (0.0 0.0) false :!label _label_2) ; Clear the drag selection box
  )
  (:`Completed`
    (goto _label_2)))

(event `EnhancedInput|/Game/Levels/Bar/Input/Actions/IA_Strategy_MoveCamera`
  (params (ActionValue :type "Vector2D Structure") (ElapsedSeconds :type "Float (double-precision)") (TriggeredSeconds :type "Float (double-precision)") (InputAction :type "InputAction Object Reference" :default "/Game/Levels/Bar/Input/Actions/IA_Strategy_MoveCamera.IA_Strategy_MoveCamera"))
  ;[0.15 0.15 0.15 0.502] Camera Logic
  ;;[0.15 0.15 0.15 0.502] Spectator Pawn Movement - our pawn is essentially a floating fixed angle camera. Because our view is 3/4, we're actually moving diagonally when it looks like we're moving straight
)

(event `EnhancedInput|/Game/Levels/Bar/Input/Actions/IA_Strategy_SelectClick`
  (params (ActionValue :type Boolean) (ElapsedSeconds :type "Float (double-precision)") (TriggeredSeconds :type "Float (double-precision)") (InputAction :type "InputAction Object Reference" :default "/Game/Levels/Bar/Input/Actions/IA_Strategy_SelectClick.IA_Strategy_SelectClick"))
  ;[0.15 0.15 0.15 0.502] Selection Logic for Mouse - Select / Drag Select on Hold
  ;;[0.15 0.15 0.15 0.502] Click Select Input (fires off on Tap)
  (:`Completed`
    (`self.Do Selection Command - Mouse`)))

(event `Do Selection Command - Mouse`
  (bind (_hit _location) (`self.GetLocationUnderCursor`))
  (bind _cachedselection (`self.CachedSelection`))
  (bind _target_unit (`self.Target Unit`))
  (bind _target_unit_2 (`self.Target Unit`))
  (bind _controlled_units (`self.Controlled Units`))
  ;[0.15 0.15 0.15 0.502] Selection Management - functionality differs if user is using a Mouse or Touchscreen
  (if _hit
    (set `self.CachedSelection` _location)
    (bind _outhit (`KismetSystemLibrary.SphereTraceSingleForObjects` _cachedselection (+ _cachedselection (0.0 0.0 350.0)) (`self.InteractionRadius`) (`|MakeArray` "ObjectTypeQuery3" :!type "EObjectTypeQuery Enum") true :!label _label_3)) ; Vertical sphere trace using the mouse location and interaction\nradius to catch any Z offset potential selectables
    (switch `/Game/Levels/Bar/Input/Enum_InputModes` (`self.InputModes`)
      (:`NewEnumerator0`
        (if (not (`self.SelectionModifier`))
          (`self.Do Deselect All Command`)))
      (:`NewEnumerator1`
        _))
    (bind (_bblockinghit _binitialoverlap _time _distance _location_2 _impactpoint _normal _impactnormal _physmat _hitactor) (`GameplayStatics.BreakHitResult` _outhit))
    (if _bblockinghit
      ;; If using selection modifier, add or remove the targeted Pawn from the array of controlled pawns, allowing for granular selectionand deselection
      (bind _output_get (set `self.Target Unit` _hitactor))
      (if (`KismetArrayLibrary.Array_Contains` _controlled_units _output_get)
        (`KismetArrayLibrary.Array_RemoveItem` _controlled_units _target_unit)
        (message `/Game/Levels/Bar/OldBlueprints/BPI_Strategy.UnitDeselected` _target_unit)
        (else
          (`KismetArrayLibrary.Array_Add` _controlled_units _target_unit_2)
          (message `/Game/Levels/Bar/OldBlueprints/BPI_Strategy.UnitSelected` _target_unit_2)))
      (else
        (switch `/Game/Levels/Bar/Input/Enum_InputModes` (`self.InputModes`)
          (:`NewEnumerator1`
            (if (`self.DoubleTapActive`)
              (set `self.DoubleTapActive` false)
              (else
                (`self.Do Move Units Command`)))))))))

(event `Do Selection Command - Touch`
  (params (CachedSelection :type "Vector Structure"))
  ;[0.15 0.15 0.15 0.502] Selection Management - functionality differs if user is using a Mouse or Touchscreen
  (set `self.CachedSelection` CachedSelection)
  (goto _label_3))

(event `EnhancedInput|/Game/Levels/Bar/Input/Actions/IA_Strategy_Zoom`
  (params (ActionValue :type "Float (double-precision)") (ElapsedSeconds :type "Float (double-precision)") (TriggeredSeconds :type "Float (double-precision)") (InputAction :type "InputAction Object Reference" :default "/Game/Levels/Bar/Input/Actions/IA_Strategy_Zoom.IA_Strategy_Zoom"))
  ;[0.15 0.15 0.15 0.502] Camera Logic
  ;;[0.15 0.15 0.15 0.502] Zoom Camera
)

(event `EnhancedInput|/Game/Levels/Bar/Input/Actions/IA_Strategy_SelectionModifier`
  (params (ActionValue :type Boolean) (ElapsedSeconds :type "Float (double-precision)") (TriggeredSeconds :type "Float (double-precision)") (InputAction :type "InputAction Object Reference" :default "/Game/Levels/Bar/Input/Actions/IA_Strategy_SelectionModifier.IA_Strategy_SelectionModifier"))
  ;[0.15 0.15 0.15 0.502] Selection Logic for Mouse - Select / Drag Select on Hold
  ;;[0.15 0.15 0.15 0.502] Selection Modifier Input - allows granular grouped unit selection
  (:`Triggered`
    (set `self.SelectionModifier` ActionValue :!label _label_4))
  (:`Canceled`
    (goto _label_4))
  (:`Completed`
    (goto _label_4)))

(event `EnhancedInput|/Game/Levels/Bar/Input/Actions/IA_Strategy_ResetCamera`
  (params (ActionValue :type Boolean) (ElapsedSeconds :type "Float (double-precision)") (TriggeredSeconds :type "Float (double-precision)") (InputAction :type "InputAction Object Reference" :default "/Game/Levels/Bar/Input/Actions/IA_Strategy_ResetCamera.IA_Strategy_ResetCamera"))
  ;[0.15 0.15 0.15 0.502] Camera Logic
  ;;[0.15 0.15 0.15 0.502] Zoom Camera
)

(event `EnhancedInput|/Game/Levels/Bar/Input/Actions/IA_Strategy_InteractHold`
  (params (ActionValue :type Boolean) (ElapsedSeconds :type "Float (double-precision)") (TriggeredSeconds :type "Float (double-precision)") (InputAction :type "InputAction Object Reference" :default "/Game/Levels/Bar/Input/Actions/IA_Strategy_InteractHold.IA_Strategy_InteractHold"))
  ;[0.15 0.15 0.15 0.502] Interaction Inputs for Mouse - Interact / Move / Drag Scroll on Hold
  (:`Triggered`
    (`self.Do Drag Scroll Command`))
  (:`Started`
    (bind _mouse_pos (`self.GetMouseLocation`))
    (set `self.StartingInteractionPosition` _mouse_pos)))

(event `EnhancedInput|/Game/Levels/Bar/Input/Actions/IA_Strategy_InteractClick`
  (params (ActionValue :type Boolean) (ElapsedSeconds :type "Float (double-precision)") (TriggeredSeconds :type "Float (double-precision)") (InputAction :type "InputAction Object Reference" :default "/Game/Levels/Bar/Input/Actions/IA_Strategy_InteractClick.IA_Strategy_InteractClick"))
  (bind (_hit _location) (`self.GetLocationUnderCursor`))
  ;[0.15 0.15 0.15 0.502] Interaction Inputs for Mouse - Interact / Move / Drag Scroll on Hold
  (:`Started`
    (`self.Reset Interaction`))
  (:`Completed`
    (if (and (> (`KismetArrayLibrary.Array_Length` (`self.Controlled Units`)) 0) _hit)
      (set `self.Cached Interaction` _location)
      (if (`self.DoubleTapActive`)
        (set `self.DoubleTapActive` false)
        (else
          (`self.Do Move Units Command`))))))

(event `Do Move Units Command`
  (bind _controlled_units (`self.Controlled Units`))
  (bind _cached_interaction (`self.Cached Interaction`))
  ;[0.15 0.15 0.15 0.502] Move to location logic for NPCs - sort by distance, move in loose formation to the location and then, if within range of the target location, attempt to interact.
  (switch `/Game/Levels/Bar/Input/Enum_InputModes` (`self.InputModes`)
    (:`NewEnumerator0`
      (set `self.CurrentMoveGoal` (`self.Cached Interaction`)))
    (:`NewEnumerator1`
      (set `self.CurrentMoveGoal` (`self.CachedSelection`))))
  (bind _closest (`self.Get Closest Actor to Location` _controlled_units (`self.CurrentMoveGoal`)))
  (set `self.InteractionFailed` false)
  (for _array_element _controlled_units
    (message `/Game/Levels/Bar/OldBlueprints/BPI_Strategy.StopMovement` _array_element)
    (`self.GroupNPCMovement` (`AIBlueprintHelperLibrary.GetAIController` _array_element) (== _array_element _closest) (`self.CurrentMoveGoal`) (* (`self.InteractionRadius`) 0.66) ; Move the first NPC in the array - the nearest to \nthe target - to the target location. Move any\nremaining NPCs to navigable locations offset\nfrom the target location by a random amount.
      (:`OnRequestFailed`
        (set `self.InteractionFailed` true))
      (:`OnMoveFinished`
        (`/Engine/EditorBlueprintResources/StandardMacros.IsValid` _array_element
          (:`Is Valid`
            (if (< (`self.2DVectorLength` (`self.K2_GetActorLocation` _array_element) (`self.Cached Interaction`)) (`self.InteractionRadius`))
              (`/Engine/EditorBlueprintResources/StandardMacros.DoOnce` false :!label _label_5
                (:`Completed`
                  (bind _outhit (`KismetSystemLibrary.SphereTraceSingleForObjects` _cached_interaction (+ _cached_interaction (0.0 0.0 350.0)) (`self.InteractionRadius`) (`|MakeArray` "ObjectTypeQuery2" "ObjectTypeQuery3" "ObjectTypeQuery4" :!type "EObjectTypeQuery Enum") true (`self.Controlled Units`)))
                  (bind (_bblockinghit _binitialoverlap _time _distance _location _impactpoint _normal _impactnormal _physmat _hitactor) (`GameplayStatics.BreakHitResult` _outhit))
                  (if _bblockinghit
                    (message `/Game/Levels/Bar/OldBlueprints/BPI_Strategy.Interact` _hitactor _array_element))))))))))
  ;; UI feedback for move success
  (`self.Cursor Feedback` (not (`self.InteractionFailed`))))

(event `Cursor Feedback`
  (params (Positive :type Boolean))
  ;[0.15 0.15 0.15 0.502] Cursor Visual Feedback
  (`NiagaraFunctionLibrary.SpawnSystemAtLocation` (select `bool` Positive :`false` "/Game/TopDown/Cursor/FX_Cursor_Failure.FX_Cursor_Failure" :`true` "/Game/TopDown/Cursor/FX_Cursor_Success.FX_Cursor_Success" :!type "NiagaraSystem Object Reference") (`self.Cached Interaction`)))

(event `Reset Interaction`
  ;[0.15 0.15 0.15 0.502] Move to location logic for NPCs - sort by distance, move in loose formation to the location and then, if within range of the target location, attempt to interact.
  (goto _label_5 :!via `Reset`))

(event `EnhancedInput|/Game/Levels/Bar/Input/Actions/IA_Strategy_Touch_PrimaryHold`
  (params (ActionValue :type "Vector2D Structure") (ElapsedSeconds :type "Float (double-precision)") (TriggeredSeconds :type "Float (double-precision)") (InputAction :type "InputAction Object Reference" :default "/Game/Levels/Bar/Input/Actions/IA_Strategy_Touch_PrimaryHold.IA_Strategy_Touch_PrimaryHold"))
  (bind (_startingsecondfingerposition_x _startingsecondfingerposition_y) (`KismetMathLibrary.BreakVector2D` (`self.StartingSecondFingerPosition`)))
  (bind (_currentinteractionposition_x _currentinteractionposition_y) (`KismetMathLibrary.BreakVector2D` (`self.CurrentInteractionPosition`)))
  ;[0.15 0.15 0.15 0.502] Touch Input - Select on Tap, second fingure selection modifier, Select All on Double Tap, Scroll Camera or Drag Select (with selection modifier) on hold.
  (:`Triggered`
    (if (and (`self.SelectionModifier`) (== (`self.StartingSecondFingerPosition`) (`self.CurrentSecondFingerPosition`) :`ErrorTolerance` 10.0))
      (set `self.CurrentInteractionPosition` ActionValue)
      (message `/Game/Levels/Bar/OldBlueprints/BPI_Strategy.DragSelectUpdate` (`self.GetHUD`) (`self.StartingInteractionPosition`) (`KismetMathLibrary.MakeVector2D` (- _currentinteractionposition_x _startingsecondfingerposition_x) (- _currentinteractionposition_y _startingsecondfingerposition_y)) (`KismetMathLibrary.MakeVector2D` _currentinteractionposition_x _currentinteractionposition_y) true)
      (else
        (`self.Do Drag Scroll Command`))))
  (:`Started`
    (set `self.StartingInteractionPosition` ActionValue)))

(event `EnhancedInput|/Game/Levels/Bar/Input/Actions/IA_Strategy_Touch_PrimaryTap`
  (params (ActionValue :type "Vector2D Structure") (ElapsedSeconds :type "Float (double-precision)") (TriggeredSeconds :type "Float (double-precision)") (InputAction :type "InputAction Object Reference" :default "/Game/Levels/Bar/Input/Actions/IA_Strategy_Touch_PrimaryTap.IA_Strategy_Touch_PrimaryTap"))
  ;[0.15 0.15 0.15 0.502] Touch Input - Select on Tap, second fingure selection modifier, Select All on Double Tap, Scroll Camera or Drag Select (with selection modifier) on hold.
  (:`Completed`
    (`self.Do Selection Command - Touch` (`self.ProjectTouchPointToWorldSpace`))))

(event `EnhancedInput|/Game/Levels/Bar/Input/Actions/IA_Strategy_Touch_Secondary`
  (params (ActionValue :type "Vector2D Structure") (ElapsedSeconds :type "Float (double-precision)") (TriggeredSeconds :type "Float (double-precision)") (InputAction :type "InputAction Object Reference" :default "/Game/Levels/Bar/Input/Actions/IA_Strategy_Touch_Secondary.IA_Strategy_Touch_Secondary"))
  ;[0.15 0.15 0.15 0.502] Touch Input - Select on Tap, second fingure selection modifier, Select All on Double Tap, Scroll Camera or Drag Select (with selection modifier) on hold.
  (:`Triggered`
    (set `self.CurrentSecondFingerPosition` ActionValue))
  (:`Started`
    (set `self.SelectionModifier` true)
    (set `self.StartingSecondFingerPosition` ActionValue))
  (:`Canceled`
    (set `self.SelectionModifier` false :!label _label_6))
  (:`Completed`
    (goto _label_6)))

(event `EnhancedInput|/Game/Levels/Bar/Input/Actions/IA_Strategy_Touch_DoubleTap`
  (params (ActionValue :type "Vector2D Structure") (ElapsedSeconds :type "Float (double-precision)") (TriggeredSeconds :type "Float (double-precision)") (InputAction :type "InputAction Object Reference" :default "/Game/Levels/Bar/Input/Actions/IA_Strategy_Touch_DoubleTap.IA_Strategy_Touch_DoubleTap"))
  ;[0.15 0.15 0.15 0.502] Touch Input - Select on Tap, second fingure selection modifier, Select All on Double Tap, Scroll Camera or Drag Select (with selection modifier) on hold.
  ;;[0.15 0.15 0.15 0.502] Select All Input (Double Tap)
  (:`Triggered`
    (set `self.DoubleTapActive` true)
    (if (`self.SelectionModifier`)
      (`self.Do Deselect All Command`)
      (else
        (`self.Do Select All On Screen Command`)))))

(fn `2DVectorLength`
  (params (VectorA :type "Vector Structure") (VectorB :type "Vector Structure"))
  (returns (Length :type "Float (double-precision)"))
  (return (`KismetMathLibrary.VSize2D` (- (`KismetMathLibrary.MakeVector2D` VectorA_X VectorA_Y) (`KismetMathLibrary.MakeVector2D` VectorB_X VectorB_Y)))))

(fn `Do Deselect All Command`
  (bind _controlled_units (`self.Controlled Units`))
  (for _array_element _controlled_units
    (`/Engine/EditorBlueprintResources/StandardMacros.IsValid` _array_element
      (:`Is Valid`
        (message `/Game/Levels/Bar/OldBlueprints/BPI_Strategy.UnitDeselected` _array_element))))
  (`KismetArrayLibrary.Array_Clear` _controlled_units)
  (return))

(fn `Do Drag Scroll Command`
  (locals (WorkingPosition :type "Vector2D Structure"))
  (bind (_locationx _locationy) (`self.GetInputTouchState` "Touch1"))
  (bind (_locationx_2 _locationy_2) (`self.GetMousePosition`))
  (bind (_returnvalue_x _returnvalue_y) (`KismetMathLibrary.BreakVector2D` (- (`self.StartingInteractionPosition`) (`local.WorkingPosition`))))
  (switch `/Game/Levels/Bar/Input/Enum_InputModes` (`self.InputModes`)
    (:`NewEnumerator0`
      (set `local.WorkingPosition` (`KismetMathLibrary.MakeVector2D` _locationx_2 _locationy_2)))
    (:`NewEnumerator1`
      (set `local.WorkingPosition` (`KismetMathLibrary.MakeVector2D` _locationx _locationy))))
  (`self.K2_AddActorWorldOffset` (`self.K2_GetPawn`) (* (`KismetMathLibrary.GreaterGreater_VectorRotator` (`KismetMathLibrary.MakeVector` _returnvalue_x _returnvalue_y) (struct :`Yaw` -45.0)) (`self.DragMultiplier`)) false false))

(fn `Do Select All On Screen Command`
  (bind _controlled_units (`self.Controlled Units`))
  (bind _outactors (`GameplayStatics.GetAllActorsOfClass` "/Script/Engine.Pawn"))
  (for _array_element _outactors
    (if (and (not (`KismetArrayLibrary.Array_Contains` _controlled_units _array_element)) (`self.WasRecentlyRendered` _array_element 0.2))
      (`KismetArrayLibrary.Array_Add` _controlled_units _array_element)
      (message `/Game/Levels/Bar/OldBlueprints/BPI_Strategy.UnitSelected` _array_element))))

(fn `DragSelectResult`
  (params (SelectedActors :type "Array of Actor Object Reference (by ref)"))
  (returns (NewParam :type Boolean))
  (if (> (`KismetArrayLibrary.Array_Length` SelectedActors) 0)
    (`self.Do Deselect All Command`)
    (for _array_element SelectedActors
      (message `/Game/Levels/Bar/OldBlueprints/BPI_Strategy.UnitSelected` _array_element)
      (`KismetArrayLibrary.Array_Add` (`self.Controlled Units`) _array_element))
    (return false)))

(fn `Get Closest Actor to Location`
  (params (ActorArray :type "Array of Actor Object Reference") (TargetLocation :type "Vector Structure"))
  (returns (Closest :type "Actor Object Reference"))
  (locals (`Out Actor` :type "Actor Object Reference") (`Closest Distance` :type "Float (double-precision)"))
  ; Process each actor on the list
  (set `local.Out Actor` null)
  (for _array_element ActorArray
    ; Have we selected a closest candidate already?
    (if (== (`local.Out Actor`) null)
      ; If we don't have an actor yet selected, choose the current one and set the closest distance.
      (bind _output_get (set `local.Out Actor` _array_element))
      (set `local.Closest Distance` (`KismetMathLibrary.Vector_DistanceSquared` (`self.K2_GetActorLocation` _output_get) (`local.TargetLocation`)))
      (else
        (bind _returnvalue (`KismetMathLibrary.Vector_DistanceSquared` (`self.K2_GetActorLocation` _array_element) (`self.K2_GetActorLocation` (`local.Out Actor`))))
        ; Check if the distance to the current actor is closer, and update the output actor and distance for the next chec.
        (if (< _returnvalue (`local.Closest Distance`))
          (set `local.Out Actor` _array_element)
          (set `local.Closest Distance` _returnvalue)))))
  ; When we're done, return the closest actor found
  (return (`local.Out Actor`)))

(fn `GetLocationUnderCursor`
  (returns (Hit :type Boolean) (Location :type "Vector Structure"))
  (bind (_bblockinghit _binitialoverlap _time _distance _location) (`GameplayStatics.BreakHitResult` (`self.GetHitResultUnderCursorByChannel` "TraceTypeQuery1")))
  (return _bblockinghit _location))

(fn `GetLocationUnderFinger`
  (returns (Hit :type Boolean) (Location :type "Vector Structure"))
  (bind (_bblockinghit _binitialoverlap _time _distance _location) (`GameplayStatics.BreakHitResult` (`self.GetHitResultUnderFingerByChannel` "Touch1" "TraceTypeQuery1" false)))
  (return _bblockinghit _location))

(fn `GetMouseLocation`
  (returns (`Mouse Pos` :type "Vector2D Structure"))
  (bind (_locationx _locationy) (`self.GetMousePosition` (`GameplayStatics.GetPlayerController` 0)))
  (return (`KismetMathLibrary.MakeVector2D` _locationx _locationy)))

(fn `PassSelectedUnits`
  (returns (Actors :type "Array of Actor Object Reference"))
  (return (`self.Controlled Units`)))

(fn `UserConstructionScript`)