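; Strategy HUD that creates the UI_Strategy widget and draws drag selection and selected-unit markers.
; The player controller feeds box geometry through DragSelectUpdate; while it is active, DrawHUD draws a translucent rectangle, gathers BP_StrategyUnit actors inside it and messages them back to the controller.
; Each frame it also fetches the controller's selected units, updates the widget count and draws a "selected" text pip at each unit's projected screen position.
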(event `self.ReceiveBeginPlay`
  ;[0.15 0.15 0.15 0.502] Setup UI
  (bind _returnvalue (`|CreateWidget` "/Game/Levels/Bar/UI/UI_Strategy.UI_Strategy_C" (`GameplayStatics.GetPlayerController` 0)))
  (bind _output_get (set `self.UI` _returnvalue))
  (`UserWidget.AddToViewport` _output_get 0))

(event `self.ReceiveDrawHUD`
  (params (SizeX :type Integer) (SizeY :type Integer))
  (bind (_start_x _start_y) (`KismetMathLibrary.BreakVector2D` (`self.Start`)))
  (bind (_widthheight_x _widthheight_y) (`KismetMathLibrary.BreakVector2D` (`self.WidthHeight`)))
  ;[0.15 0.15 0.15 0.502] Drag Select Logic - take selection rectangle width, height and position from Player Controller, draw a rectangle on the HUD to match
  (`|ExecutionSequence`
    (:`then_0`
      (if (`self.DrawBox`)
        (`self.DrawRect` (struct :`R` 1.0 :`G` 1.0 :`B` 1.0 :`A` 0.5) _start_x _start_y _widthheight_x _widthheight_y)
        (bind _output_get (set `self.SelectedActors` (`self.GetActorsInSelectionRectangle` "/Game/Levels/Bar/OldBlueprints/BP_StrategyUnit.BP_StrategyUnit_C" (`self.Start`) (`self.CurrentPosition`))))
        (message `/Game/Levels/Bar/OldBlueprints/BPI_Strategy.DragSelectResult` (`GameplayStatics.GetPlayerController` 0) _output_get)))
    (:`then_1`
      ;[0.15 0.15 0.15 0.502] A simple routine to draw selection pips on the characters.
      (bind _actors (message `/Game/Levels/Bar/OldBlueprints/BPI_Strategy.PassSelectedUnits` (`GameplayStatics.GetPlayerController` 0)))
      (bind _returnvalue (`KismetArrayLibrary.Array_Length` _actors))
      (`/Game/Levels/Bar/UI/UI_Strategy.Set Selected Units Count` (`self.UI`) _returnvalue)
      (if (> _returnvalue 0)
        (for _array_element _actors
          (bind _screenposition (`GameplayStatics.ProjectWorldToScreen` (`GameplayStatics.GetPlayerController` 0) (`self.K2_GetActorLocation` _array_element) true))
          (`self.DrawSelectionPip` "selected" (`KismetMathLibrary.BreakVector2D` _screenposition) (`.Y` (`KismetMathLibrary.BreakVector2D` _screenposition)) 25.0 25.0))))))

(event `/Game/Levels/Bar/OldBlueprints/BPI_Strategy.DragSelectUpdate`
  (params (Start :type "Vector2D Structure") (`Width and Height` :type "Vector2D Structure") (CurrentPosition :type "Vector2D Structure") (Draw :type Boolean))
  ;[0.15 0.15 0.15 0.502] Drag Select Logic - take selection rectangle width, height and position from Player Controller, draw a rectangle on the HUD to match
  ;;[0.15 0.15 0.15 0.502] Data Update from Player Controller
  (set `self.DrawBox` Draw)
  (set `self.Start` Start)
  (set `self.WidthHeight` `Width and Height`)
  (set `self.CurrentPosition` CurrentPosition))

(fn `DragSelectResult`
  (params (SelectedActors :type "Array of Actor Object Reference (by ref)"))
  (returns (NewParam :type Boolean))
  (return false))

(fn `DrawSelectionPip`
  (params (Text :type String) (X :type "Float (double-precision)") (Y :type "Float (double-precision)") (`Bounds X` :type "Float (double-precision)") (`Bounds Y` :type "Float (double-precision)"))
  (`self.DrawText` Text (struct :`R` 1.0 :`G` 1.0 :`B` 1.0 :`A` 1.0) (- X `Bounds X`) (+ Y `Bounds Y`) null 1.5))

(fn `PassSelectedUnits`
  (returns (Actors :type "Array of Actor Object Reference"))
  (return))

(fn `UserConstructionScript`)