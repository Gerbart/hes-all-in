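; BP_StrategyUnit is a selectable character unit for strategy-style play, randomized to the Manny mesh about half the time at construction.
; It exposes stop, selection and material hooks, while its drag-select and pass-units functions are empty stubs.
; On Interact it turns toward the interactor and both units play their response animation.
; Selection or the animation's end switches the mesh back to its Animation Blueprint.
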(event `/Game/Levels/OldBar/OldBlueprints/BPI_Strategy.StopMovement`
  ; Stop Moving
  (`MovementComponent.StopMovementImmediately` (`self.CharacterMovement`)))

(event `/Game/Levels/OldBar/OldBlueprints/BPI_Strategy.UnitSelected`
  ; Reset Animation when Selected
  (if (`|EnumInequality` (`SkeletalMeshComponent.GetAnimationMode` (`self.Mesh`)) "AnimationBlueprint")
    (`SkeletalMeshComponent.SetAnimationMode` (`self.Mesh`) "AnimationBlueprint" true)))

(event `/Game/Levels/OldBar/OldBlueprints/BPI_Strategy.Interact`
  (params (Interactor :type "Actor Object Reference"))
  ; Interaction Event, activated upon receiving Interact message via Interface. Plays an animation.
  (`|ExecutionSequence`
    (:`then_0`
      (`self.K2_SetActorRotation` (`KismetMathLibrary.FindLookAtRotation` (`self.K2_GetActorLocation`) (`self.K2_GetActorLocation` Interactor)))
      (`self.Interaction Behavior`))
    (:`then_1`
      (bind _asbp_strategy_unit (cast `/Game/Levels/OldBar/OldBlueprints/BP_StrategyUnit` Interactor))
      (`self.Interaction Behavior` _asbp_strategy_unit))))

(event `Interaction Behavior`
  (bind _mesh (`self.Mesh`))
  (bind _responseanimation (`self.ResponseAnimation`))
  ; Interaction Event, activated upon receiving Interact message via Interface. Plays an animation.
  (`SkeletalMeshComponent.PlayAnimation` _mesh _responseanimation false)
  (`KismetSystemLibrary.Delay` (`AnimationAsset.GetPlayLength` _responseanimation))
  (`SkeletalMeshComponent.SetAnimationMode` _mesh "AnimationBlueprint" true))

(fn `DragSelectResult`
  (params (SelectedActors :type "Array of Actor Object Reference (by ref)"))
  (returns (NewParam :type Boolean))
  (return false))

(fn `PassSelectedUnits`
  (returns (Actors :type "Array of Actor Object Reference"))
  (return))

(fn `SetMaterial`
  (params (Material :type "MaterialInterface Object Reference"))
  (bind _mesh (`self.Mesh`))
  (`PrimitiveComponent.SetMaterial` _mesh 0 Material)
  (`PrimitiveComponent.SetMaterial` _mesh 1 Material))

(fn `UserConstructionScript`
  ;[0.15 0.15 0.15 0.502] Randomize NPC, they have a 50/50 chance of being Manny or Quinn
  (if (> (`KismetMathLibrary.RandomIntegerInRange` 0 100) 50)
    (set `SkeletalMeshComponent.SkeletalMeshAsset` "/Game/Characters/Mannequins/Meshes/SKM_Manny_Simple.SKM_Manny_Simple" (`self.Mesh`))))