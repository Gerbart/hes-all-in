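; Cutscene actor for the Charlie's Scene transition level that plays an audio track with timed dialogue text, then loads ReggiesScene.
; On BeginPlay it starts the Audio component and adds a WBP_Dialogue widget showing the first entry of the Lines array.
; A hardcoded chain of Delays steps CurrentLine through the array, updating the widget's text at each step.
; The level opens immediately after the last line is set, with no final delay.
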(event `self.ReceiveBeginPlay`
  (`AudioComponent.Play` (`self.Audio`) 0.0)
  (bind _returnvalue (`|CreateWidget` "/Game/Gamemode/Blueprints/WBP_Dialogue.WBP_Dialogue_C"))
  (set `/Game/Gamemode/Blueprints/WBP_Dialogue.String` (`|GetArrayItem` (`self.Lines`) (`self.Current Line`)) _returnvalue)
  (bind _output_get (set `self.Dialogue Widget` _returnvalue))
  (`UserWidget.AddToViewport` _output_get 0)
  (`KismetSystemLibrary.Delay` 1.0)
  (bind _result (`/Engine/EditorBlueprintResources/StandardMacros.IncrementInt` (`self.Current Line`))
    (:`  `
      (set `self.Current Line` _result)
      (set `/Game/Gamemode/Blueprints/WBP_Dialogue.String` (`|GetArrayItem` (`self.Lines`) (`self.Current Line`)) (`self.Dialogue Widget`))
      (`KismetSystemLibrary.Delay` 2.0)
      (bind _result_2 (`/Engine/EditorBlueprintResources/StandardMacros.IncrementInt` (`self.Current Line`))
        (:`  `
          (set `self.Current Line` _result_2)
          (set `/Game/Gamemode/Blueprints/WBP_Dialogue.String` (`|GetArrayItem` (`self.Lines`) (`self.Current Line`)) (`self.Dialogue Widget`))
          (`KismetSystemLibrary.Delay` 6.0)
          (bind _result_3 (`/Engine/EditorBlueprintResources/StandardMacros.IncrementInt` (`self.Current Line`))
            (:`  `
              (set `self.Current Line` _result_3)
              (set `/Game/Gamemode/Blueprints/WBP_Dialogue.String` (`|GetArrayItem` (`self.Lines`) (`self.Current Line`)) (`self.Dialogue Widget`))
              (`KismetSystemLibrary.Delay` 2.0)
              (bind _result_4 (`/Engine/EditorBlueprintResources/StandardMacros.IncrementInt` (`self.Current Line`))
                (:`  `
                  (set `self.Current Line` _result_4)
                  (set `/Game/Gamemode/Blueprints/WBP_Dialogue.String` (`|GetArrayItem` (`self.Lines`) (`self.Current Line`)) (`self.Dialogue Widget`))
                  (`KismetSystemLibrary.Delay` 2.0)
                  (bind _result_5 (`/Engine/EditorBlueprintResources/StandardMacros.IncrementInt` (`self.Current Line`))
                    (:`  `
                      (set `self.Current Line` _result_5)
                      (set `/Game/Gamemode/Blueprints/WBP_Dialogue.String` (`|GetArrayItem` (`self.Lines`) (`self.Current Line`)) (`self.Dialogue Widget`))
                      (`KismetSystemLibrary.Delay` 2.5)
                      (bind _result_6 (`/Engine/EditorBlueprintResources/StandardMacros.IncrementInt` (`self.Current Line`))
                        (:`  `
                          (set `self.Current Line` _result_6)
                          (set `/Game/Gamemode/Blueprints/WBP_Dialogue.String` (`|GetArrayItem` (`self.Lines`) (`self.Current Line`)) (`self.Dialogue Widget`))
                          (`KismetSystemLibrary.Delay` 2.0)
                          (bind _result_7 (`/Engine/EditorBlueprintResources/StandardMacros.IncrementInt` (`self.Current Line`))
                            (:`  `
                              (set `self.Current Line` _result_7)
                              (set `/Game/Gamemode/Blueprints/WBP_Dialogue.String` (`|GetArrayItem` (`self.Lines`) (`self.Current Line`)) (`self.Dialogue Widget`))
                              (`KismetSystemLibrary.Delay` 3.5)
                              (bind _result_8 (`/Engine/EditorBlueprintResources/StandardMacros.IncrementInt` (`self.Current Line`))
                                (:`  `
                                  (set `self.Current Line` _result_8)
                                  (set `/Game/Gamemode/Blueprints/WBP_Dialogue.String` (`|GetArrayItem` (`self.Lines`) (`self.Current Line`)) (`self.Dialogue Widget`))
                                  (`KismetSystemLibrary.Delay` 6.0)
                                  (bind _result_9 (`/Engine/EditorBlueprintResources/StandardMacros.IncrementInt` (`self.Current Line`))
                                    (:`  `
                                      (set `self.Current Line` _result_9)
                                      (set `/Game/Gamemode/Blueprints/WBP_Dialogue.String` (`|GetArrayItem` (`self.Lines`) (`self.Current Line`)) (`self.Dialogue Widget`))
                                      (`KismetSystemLibrary.Delay` 2.5)
                                      (bind _result_10 (`/Engine/EditorBlueprintResources/StandardMacros.IncrementInt` (`self.Current Line`))
                                        (:`  `
                                          (set `self.Current Line` _result_10)
                                          (set `/Game/Gamemode/Blueprints/WBP_Dialogue.String` (`|GetArrayItem` (`self.Lines`) (`self.Current Line`)) (`self.Dialogue Widget`))
                                          (`KismetSystemLibrary.Delay` 1.0)
                                          (bind _result_11 (`/Engine/EditorBlueprintResources/StandardMacros.IncrementInt` (`self.Current Line`))
                                            (:`  `
                                              (set `self.Current Line` _result_11)
                                              (set `/Game/Gamemode/Blueprints/WBP_Dialogue.String` (`|GetArrayItem` (`self.Lines`) (`self.Current Line`)) (`self.Dialogue Widget`))
                                              (`KismetSystemLibrary.Delay` 10.5)
                                              (bind _result_12 (`/Engine/EditorBlueprintResources/StandardMacros.IncrementInt` (`self.Current Line`))
                                                (:`  `
                                                  (set `self.Current Line` _result_12)
                                                  (set `/Game/Gamemode/Blueprints/WBP_Dialogue.String` (`|GetArrayItem` (`self.Lines`) (`self.Current Line`)) (`self.Dialogue Widget`))
                                                  (`KismetSystemLibrary.Delay` 4.0)
                                                  (bind _result_13 (`/Engine/EditorBlueprintResources/StandardMacros.IncrementInt` (`self.Current Line`))
                                                    (:`  `
                                                      (set `self.Current Line` _result_13)
                                                      (set `/Game/Gamemode/Blueprints/WBP_Dialogue.String` (`|GetArrayItem` (`self.Lines`) (`self.Current Line`)) (`self.Dialogue Widget`))
                                                      (`KismetSystemLibrary.Delay` 3.0)
                                                      (bind _result_14 (`/Engine/EditorBlueprintResources/StandardMacros.IncrementInt` (`self.Current Line`))
                                                        (:`  `
                                                          (set `self.Current Line` _result_14)
                                                          (set `/Game/Gamemode/Blueprints/WBP_Dialogue.String` (`|GetArrayItem` (`self.Lines`) (`self.Current Line`)) (`self.Dialogue Widget`))
                                                          (`KismetSystemLibrary.Delay` 21.0)
                                                          (bind _result_15 (`/Engine/EditorBlueprintResources/StandardMacros.IncrementInt` (`self.Current Line`))
                                                            (:`  `
                                                              (set `self.Current Line` _result_15)
                                                              (set `/Game/Gamemode/Blueprints/WBP_Dialogue.String` (`|GetArrayItem` (`self.Lines`) (`self.Current Line`)) (`self.Dialogue Widget`))
                                                              (`KismetSystemLibrary.Delay` 9.0)
                                                              (bind _result_16 (`/Engine/EditorBlueprintResources/StandardMacros.IncrementInt` (`self.Current Line`))
                                                                (:`  `
                                                                  (set `self.Current Line` _result_16)
                                                                  (set `/Game/Gamemode/Blueprints/WBP_Dialogue.String` (`|GetArrayItem` (`self.Lines`) (`self.Current Line`)) (`self.Dialogue Widget`))
                                                                  (`KismetSystemLibrary.Delay` 5.0)
                                                                  (bind _result_17 (`/Engine/EditorBlueprintResources/StandardMacros.IncrementInt` (`self.Current Line`))
                                                                    (:`  `
                                                                      (set `self.Current Line` _result_17)
                                                                      (set `/Game/Gamemode/Blueprints/WBP_Dialogue.String` (`|GetArrayItem` (`self.Lines`) (`self.Current Line`)) (`self.Dialogue Widget`))
                                                                      (`GameplayStatics.OpenLevel` "ReggiesScene"))))))))))))))))))))))))))))))))))))

(fn `UserConstructionScript`)